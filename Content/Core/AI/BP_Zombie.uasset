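; BP_Zombie is a zombie AI character with a fixed walk speed and a montage-driven melee attack.
; BeginPlay sets the CharacterMovement max walk speed, and Tick reapplies it every frame after printing the current velocity magnitude as debug output.
; MeleeAttack plays AttackMontage and returns the montage duration truncated to an integer.
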(event `self.ReceiveBeginPlay`
  (set `CharacterMovementComponent.MaxWalkSpeed` 300.0 (`self.CharacterMovement`) :!label _label))

(event `self.ReceiveTick`
  (params (DeltaSeconds :type "Float (single-precision)"))
  (`KismetSystemLibrary.PrintString` (`KismetStringLibrary.Conv_DoubleToString` (`KismetMathLibrary.VSize` (`self.GetVelocity`))) true true (struct :`G` 0.66 :`B` 1.0 :`A` 1.0) 0.0)
  (goto _label))

(fn `MeleeAttack`
  (returns (ReturnValue :type Integer))
  (bind _returnvalue (`self.PlayAnimMontage` (`self.AttackMontage`)))
  (return (`KismetMathLibrary.FTrunc` _returnvalue)))

(fn `UserConstructionScript`)