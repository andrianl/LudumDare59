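; BP_FinalGate is an end-of-game trigger actor that finishes the game when the player reaches it after picking up the cat.
; On BeginPlay it caches the BP_HorrorCharacter as the player.
; When that player overlaps the Box with CatPicked set, it adds the WBP_EndGame widget to the viewport, waits a fixed delay, then opens the main menu level.
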(event `self.ReceiveBeginPlay`
  (bind _returnvalue (`GameplayStatics.GetActorOfClass` "/Game/Core/Variant_Horror/Blueprints/BP_HorrorCharacter.BP_HorrorCharacter_C"))
  (set `self.Player` _returnvalue))

(event `self.Box.OnComponentBeginOverlap`
  (params (OverlappedComponent :type "PrimitiveComponent Object Reference") (OtherActor :type "Actor Object Reference") (OtherComp :type "PrimitiveComponent Object Reference") (OtherBodyIndex :type Integer) (bFromSweep :type Boolean) (SweepResult :type "HitResult Structure (by ref)"))
  (bind _player (`self.Player`))
  (if (and (== OtherActor _player) (`/Game/Core/Variant_Horror/Blueprints/BP_HorrorCharacter.CatPicked` _player))
    (bind _returnvalue (`|CreateWidget` "/Game/Core/MainMenu/WBP_EndGame.WBP_EndGame_C" (`GameplayStatics.GetPlayerController` 0)))
    (`UserWidget.AddToViewport` _returnvalue 0)
    (`KismetSystemLibrary.Delay` 10.0)
    (`GameplayStatics.OpenLevelBySoftObjectPtr` "/Game/Maps/L_MainMenu.L_MainMenu")))

(fn `UserConstructionScript`)