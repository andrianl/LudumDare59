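; BP_SoundGenerator is a short-lived actor that visualizes a sound as an expanding ring pulse from its location, then destroys itself.
; Timelines drive radius and intensity on a dynamic post-process material, added to the level's PostProcessVolume, and on a ring decal material instance.
; After expansion it removes the decal, waits, fades the post effect and unregisters it.
; The construction script's SetDecalMaterial call is disconnected, so that instance is never assigned here.
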(event `self.ReceiveBeginPlay`
  (bind _returnvalue (* (`self.SoundRange`) 0.01))
  (bind _weightedblendables_array (break `WeightedBlendables` (break `PostProcessSettings` (`PostProcessVolume.Settings` (`self.PostProcessVolume`)))))
  (bind _returnvalue_2 (`GameplayStatics.GetActorOfClass` "/Script/Engine.PostProcessVolume"))
  (set `self.PostProcessVolume` _returnvalue_2)
  (bind _returnvalue_3 (`KismetMaterialLibrary.CreateDynamicMaterialInstance` "/Game/Core/Echo/M_Post_Add.M_Post_Add"))
  (set `self.PostProcessMaterial` _returnvalue_3)
  (`SceneComponent.SetRelativeScale3D` (`self.Decal`) (`KismetMathLibrary.MakeVector` _returnvalue _returnvalue _returnvalue))
  (`self.CE_Expand`)
  (`MaterialInstanceDynamic.SetVectorParameterValue` (`self.PostProcessMaterial`) "Location" (`KismetMathLibrary.Conv_VectorToLinearColor` (`self.K2_GetActorLocation`)))
  (`KismetArrayLibrary.Array_Add` _weightedblendables_array (make `WeightedBlendable` 1.0 (`self.PostProcessMaterial`))))

(event `CE_Expand`
  (bind (_direction _radius _intensity _intensity_decal) (`Timeline|TL_Decal` :!via `PlayFromStart`)
    (:`Update`
      (`self.UpdateRadius` (`KismetMathLibrary.Lerp` (`self.StartRange`) (`self.SoundRange`) _radius))
      (`MaterialInstanceDynamic.SetScalarParameterValue` (`self.PostProcessMaterial`) "Intensity" _intensity)
      (`MaterialInstanceDynamic.SetScalarParameterValue` (`self.MI_Decal`) "Intensity" _intensity_decal))
    (:`Finished`
      (`ActorComponent.K2_DestroyComponent` (`self.Decal`))
      (`KismetSystemLibrary.Delay` 2.0)
      (`self.CE_Finish`))))

(event `CE_Finish`
  (bind _weightedblendables_array (break `WeightedBlendables` (break `PostProcessSettings` (`PostProcessVolume.Settings` (`self.PostProcessVolume`)))))
  (bind (_direction _intensity) (`Timeline|TL_Fade`)
    (:`Update`
      (`MaterialInstanceDynamic.SetScalarParameterValue` (`self.PostProcessMaterial`) "Intensity" _intensity))
    (:`Finished`
      (`KismetArrayLibrary.Array_RemoveItem` _weightedblendables_array (make `WeightedBlendable` 1.0 (`self.PostProcessMaterial`)))
      (`self.K2_DestroyActor`))))

(fn `UpdateRadius`
  (params (Radius :type "Float (double-precision)"))
  (`MaterialInstanceDynamic.SetScalarParameterValue` (`self.PostProcessMaterial`) "Radius" Radius)
  (`MaterialInstanceDynamic.SetScalarParameterValue` (`self.MI_Decal`) "Radius" Radius))

(fn `UserConstructionScript`
  (locals (NewLocalVar :type "Vector Structure" :default (0.0 0.0 0.0)))
  (bind _returnvalue (`KismetMaterialLibrary.CreateDynamicMaterialInstance` "/Game/Core/Echo/M_RingDecal.M_RingDecal"))
  (bind _output_get (set `self.MI_Decal` _returnvalue))
  (`MaterialInstanceDynamic.SetVectorParameterValue` _output_get "Color" (`self.Decal Color`))
  (`MaterialInstanceDynamic.SetVectorParameterValue` (`self.MI_Decal`) "Location" (`KismetMathLibrary.Conv_VectorToLinearColor` (`self.K2_GetActorLocation`))))