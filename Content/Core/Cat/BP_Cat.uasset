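; BP_Cat is a cat actor that can be picked up, with a widget showing pickup progress.
; Any overlap with its PresenceSphere unhides the widget, and the end of an overlap hides it again.
; OnPickupProgressUpdate feeds the incoming progress value into the progress bar of the WBP_TakeProgress widget.
; OnCatPickedUp destroys the actor, while the pickup timing itself is driven from outside this graph.
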(event `self.OnCatPickedUp`
  (`self.K2_DestroyActor`))

(event `self.PresenceSphere.OnComponentBeginOverlap`
  (params (OverlappedComponent :type "PrimitiveComponent Object Reference") (OtherActor :type "Actor Object Reference") (OtherComp :type "PrimitiveComponent Object Reference") (OtherBodyIndex :type Integer) (bFromSweep :type Boolean) (SweepResult :type "HitResult Structure (by ref)"))
  (`SceneComponent.SetHiddenInGame` (`self.Widget`) false true))

(event `self.PresenceSphere.OnComponentEndOverlap`
  (params (OverlappedComponent :type "PrimitiveComponent Object Reference") (OtherActor :type "Actor Object Reference") (OtherComp :type "PrimitiveComponent Object Reference") (OtherBodyIndex :type Integer))
  (`SceneComponent.SetHiddenInGame` (`self.Widget`) true true))

(event `self.OnPickupProgressUpdate`
  (params (Progress :type "Float (single-precision)"))
  (bind _aswbp_take_progress (cast `/Game/Core/Cat/WBP_TakeProgress` (`WidgetComponent.GetUserWidgetObject` (`self.Widget`))))
  (`ProgressBar.SetPercent` (`/Game/Core/Cat/WBP_TakeProgress.GetProgressBar` _aswbp_take_progress) Progress))

(fn `UserConstructionScript`)